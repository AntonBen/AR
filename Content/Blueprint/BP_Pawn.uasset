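; AR pawn that opens the StartPage widget in UI-only input mode on BeginPlay and exercises device location and AR tracking.
; A looping timer calls GetGpsPos, which checks and starts location services, then prints the last known longitude or a failure message.
; Every Tick, it debug-draws all AR tracked geometries.
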(event `self.ReceiveBeginPlay`
  (bind _returnvalue (`GameplayStatics.GetPlayerController` 0))
  (bind _returnvalue_2 (`|CreateWidget` "/Game/UI/StartPage.StartPage_C" _returnvalue))
  (`UserWidget.AddToViewport` _returnvalue_2 0)
  (`WidgetBlueprintLibrary.SetInputMode_UIOnlyEx` _returnvalue null)
  (`KismetSystemLibrary.K2_SetTimer` null "GetGpsPos" 7.0 true))

(event `GetGpsPos`
  (bind _returnvalue (`LocationServices.AreLocationServicesEnabled`))
  (if _returnvalue
    (bind _returnvalue_2 (`LocationServices.StartLocationServices`))
    (if _returnvalue_2
      (bind _returnvalue_3 (`LocationServices.GetLastKnownLocation`))
      (`KismetSystemLibrary.PrintText` (`KismetTextLibrary.Conv_StringToText` (`KismetStringLibrary.Conv_DoubleToString` (`.Longitude` (break `LocationServicesData` _returnvalue_3)))))
      (else
        (`KismetSystemLibrary.PrintString` "service not ready ")))
    (else
      (`KismetSystemLibrary.PrintString` "Location service is disable"))))

(event `self.ReceiveTick`
  (params (DeltaSeconds :type "Float (single-precision)"))
  (bind _returnvalue (`ARBlueprintLibrary.GetAllGeometries`))
  (for _array_element _returnvalue
    (`ARBlueprintLibrary.DebugDrawTrackedGeometry` _array_element (struct :`R` 1.0 :`G` 0.055358 :`A` 0.75))))

(fn `UserConstructionScript`)